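; A spline-driven fence Blueprint, likely chain-link given its folder, that lays spline mesh segments along an editable path.
; The Construction Script derives the loop count from spline length divided by EndLength, adding a collision-enabled, X-forward mesh per iteration.
; Segments are spaced by a separate Length value, with tangents clamped to it and each end extended slightly to overlap the next.
; The event graph has no active logic.
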(fn `UserConstructionScript`
  (bind _spline (`self.Spline`))
  (for _index (range (+ (`KismetMathLibrary.FTrunc` (/ (`SplineComponent.GetSplineLength` (`self.Spline`)) (`self.EndLength`))) 1))
    (bind _returnvalue (`AddComponent|NODE_AddSplineMeshComponent-0`))
    (`SplineMeshComponent.SetForwardAxis` _returnvalue "X" true)
    (`PrimitiveComponent.SetCollisionEnabled` _returnvalue "QueryAndPhysics")
    (bind _returnvalue_2 (* _index (`self.Length`)))
    (bind _returnvalue_3 (+ (* (+ _index 1) (`self.Length`)) 10.0))
    (`SplineMeshComponent.SetStartAndEnd` _returnvalue (`SplineComponent.GetLocationAtDistanceAlongSpline` _spline _returnvalue_2 "Local") (`KismetMathLibrary.ClampVectorSize` (`SplineComponent.GetTangentAtDistanceAlongSpline` _spline _returnvalue_2 "Local") 0.0 (`self.Length`)) (`SplineComponent.GetLocationAtDistanceAlongSpline` _spline _returnvalue_3 "Local") (`KismetMathLibrary.ClampVectorSize` (`SplineComponent.GetTangentAtDistanceAlongSpline` _spline _returnvalue_3 "Local") 0.0 (`self.Length`)) true)))